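; BP_Grid is a grid actor that builds square, hexagon or triangle tile layouts as instances on one InstancedStaticMesh.
; SpawnGrid stores its parameters, clears old instances, applies the shape's mesh and material, then snaps the center and derives the bottom-left corner.
; Per-index helpers place and rotate tiles, with hexagons stepping Y by two in staggered columns.
; Optional sphere traces snap tile height to hit ground and skip tiles without hits.
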(event EventBeginPlay)

(event Collision|EventActorBeginOverlap
  (params (OtherActor :type Actor%20Object%20Reference)))

(event EventTick
  (params (DeltaSeconds :type Float%20%28single-precision%29)))

(fn ConstructionScript)

(fn SpawnGrid
  (params (center_location :type Vector) (tile_size :type Vector) (tile_count :type Int%20Point%20Structure) (shape :type E_GridShape%20Enum :default "NewEnumerator0") (use_environment :type Boolean))
  (bind _returnvalue (CallFunction|GetCurrentShapeData))
  (bind _instancedstaticmesh (Variables|Default|GetInstancedStaticMesh))
  (bind (_mesh_size _mesh _mesh_material _flat_mesh _flat_border_material) (Utilities|Struct|BreakS_GridShapeData _returnvalue))
  ;[1 1 1] save vairables for later
  ; round the tile counts
  (Variables|Default|Setgrid_center_location center_location)
  (Variables|Default|Setgrid_tile_size tile_size)
  (Variables|Default|Setgrid_shape shape)
  (Variables|Default|Setgrid_tile_count tile_count)
  ;[1 1 1] clean up old grid
  (CallFunction|DestroyGrid)
  ;[1 1 1] set grids visual
  (Components|StaticMesh|SetStaticMesh _instancedstaticmesh _flat_mesh)
  (Rendering|Material|SetMaterial _instancedstaticmesh 0 _flat_border_material)
  (CallFunction|SetGridOffsetfromGround (Variables|Default|Getgrid_offset_from_ground))
  ;[1 1 1] determine bottom left tile location from tile size, tile count, and grid center
  (bind (_center _bottom_left) (CallFunction|CalculateCenterandBottomLeft))
  (Variables|Default|Setgrid_center_location _center)
  (Variables|Default|Setgrid_bottom_left_corner_location _bottom_left)
  ;[1 1 1] get x and y iterators
  (for _index (range 0 (- (.x (Variables|Default|Getgrid_tile_count)) 1))
    (LocalVariables|Setx _index)
    ;[1 1 1] switch depending on grid_shape: zipping up the y axis is different for hexagons (logic branch on bottom)
    (if (Utilities|Enum|NotEqual(Enum) (Variables|Default|Getgrid_shape) "NewEnumerator2")
      (for _index_2 (range 0 (- (.y (Variables|Default|Getgrid_tile_count)) 1))
        (LocalVariables|Sety _index_2)
        ;[1 1 1] set a local index pair
        (LocalVariables|Setindex (Utilities|Struct|MakeIntPoint (LocalVariables|Getx) (LocalVariables|Gety)))
        ;[1 1 1] use x,y iterators of tile grid to set each tiles transform location
        (LocalVariables|Settile_transform (Math|Transform|MakeTransform (CallFunction|GetTileLocationfromGridIndex (LocalVariables|Getindex)) (CallFunction|GetTileRotationfromGridIndex (LocalVariables|Getindex)) (/ (Variables|Default|Getgrid_tile_size) (.mesh_size (Utilities|Struct|BreakS_GridShapeData (CallFunction|GetCurrentShapeData))))))
        ;[1 1 1] if the use_environment flag is true, have the grid trace the ground. else just generate the grid tile in flatness.
        (if use_environment
          (bind (_hit_something _out_location) (CallFunction|TraceforGround (.location (LocalVariables|Gettile_transform))))
          (if _hit_something
            (LocalVariables|Settile_transform (Math|Transform|MakeTransform _out_location (.rotation (LocalVariables|Gettile_transform)) (.scale (LocalVariables|Gettile_transform))))
            ;[1 1 1] add the static mesh tile instance
            (Components|InstancedStaticMesh|AddInstance (Variables|Default|GetInstancedStaticMesh) (LocalVariables|Gettile_transform) false))
          (else
            (Components|InstancedStaticMesh|AddInstance (Variables|Default|GetInstancedStaticMesh) (LocalVariables|Gettile_transform) false))))
      (else
        (for _index_3 (range (Math|Integer|SelectInt 0 1 (CallFunction|IsIntEven (LocalVariables|Getx))) (- (* (.y (Variables|Default|Getgrid_tile_count)) 2) 1))
          (LocalVariables|Sety _index_3)
          (Utilities|FlowControl|Sequence
            (:then_0
              (LocalVariables|Setindex (Utilities|Struct|MakeIntPoint (LocalVariables|Getx) (LocalVariables|Gety)))
              (LocalVariables|Settile_transform (Math|Transform|MakeTransform (CallFunction|GetTileLocationfromGridIndex (LocalVariables|Getindex)) (CallFunction|GetTileRotationfromGridIndex (LocalVariables|Getindex)) (/ (Variables|Default|Getgrid_tile_size) (.mesh_size (Utilities|Struct|BreakS_GridShapeData (CallFunction|GetCurrentShapeData))))))
              (if use_environment
                (bind (_hit_something_2 _out_location_2) (CallFunction|TraceforGround (.location (LocalVariables|Gettile_transform))))
                (if _hit_something_2
                  (LocalVariables|Settile_transform (Math|Transform|MakeTransform _out_location_2 (.rotation (LocalVariables|Gettile_transform)) (.scale (LocalVariables|Gettile_transform))))
                  (Components|InstancedStaticMesh|AddInstance (Variables|Default|GetInstancedStaticMesh) (LocalVariables|Gettile_transform) false))
                (else
                  (Components|InstancedStaticMesh|AddInstance (Variables|Default|GetInstancedStaticMesh) (LocalVariables|Gettile_transform) false))))
            (:then_1
              (Math|Integer|IncrementInt _index_3))))))))

(fn GetCurrentShapeData
  (return (CallFunction|GetShapeData (Variables|Default|Getgrid_shape))))

(fn DestroyGrid
  (Components|InstancedStaticMesh|ClearInstances (Variables|Default|GetInstancedStaticMesh)))

(fn CalculateCenterandBottomLeft
  (bind _grid_tile_count (Variables|Default|Getgrid_tile_count))
  (switch Utilities|FlowControl|Switch|SwitchonE_GridShape (Variables|Default|Getgrid_shape)
    (:NewEnumerator1
      (LocalVariables|Setcenter_of_grid (CallFunction|SnapVectortoVector (Variables|Default|Getgrid_center_location) (Variables|Default|Getgrid_tile_size)))
      (return (LocalVariables|Getcenter_of_grid) (- (LocalVariables|Getcenter_of_grid) (* (Math|Conversions|ToVector(Vector2D) (/ (- (Math|Conversions|ToVector2D(IntPoint) (Variables|Default|Getgrid_tile_count)) (Math|Vector2D|MakeVector2D (Math|Float|SelectFloat 0.0 1.0 (CallFunction|IsIntEven (.x _grid_tile_count))) (Math|Float|SelectFloat 0.0 1.0 (CallFunction|IsIntEven (.y _grid_tile_count))))) "(X=2.000000,Y=2.000000)")) (Variables|Default|Getgrid_tile_size)))))
    (:NewEnumerator2
      (LocalVariables|Setcenter_of_grid (CallFunction|SnapVectortoVector (Variables|Default|Getgrid_center_location) (* (Variables|Default|Getgrid_tile_size) "1.500000,1.000000,1.000000")))
      (return (LocalVariables|Getcenter_of_grid) (- (LocalVariables|Getcenter_of_grid) (CallFunction|SnapVectortoVector (* (Math|Conversions|ToVector(Vector2D) (/ (Math|Conversions|ToVector2D(IntPoint) (Variables|Default|Getgrid_tile_count)) "(X=3.000000,Y=2.000000)")) (Variables|Default|Getgrid_tile_size)) (* (Variables|Default|Getgrid_tile_size) "1.500000,1.000000,1.000000")))))
    (:NewEnumerator3
      (LocalVariables|Setcenter_of_grid (CallFunction|SnapVectortoVector (Variables|Default|Getgrid_center_location) (* (Variables|Default|Getgrid_tile_size) "2.000000,1.000000,1.000000")))
      (return (LocalVariables|Getcenter_of_grid) (- (LocalVariables|Getcenter_of_grid) (CallFunction|SnapVectortoVector (* (Math|Conversions|ToVector(Vector2D) (/ (- (Math|Conversions|ToVector2D(IntPoint) (Variables|Default|Getgrid_tile_count)) "(X=1.000000,Y=1.000000)") "(X=2.000000,Y=4.000000)")) (Variables|Default|Getgrid_tile_size)) (* (Variables|Default|Getgrid_tile_size) "2.000000,1.000000,1.000000")))))))

(fn GetTileRotationfromGridIndex
  (params (grid_index :type Int%20Point%20Structure))
  (if (Utilities|Enum|Equal(Enum) (Variables|Default|Getgrid_shape) "NewEnumerator3")
    (return (Math|Rotator|MakeRotator 0.0 0.0 (+ (Math|Float|SelectFloat 1.8e+02 0.0 (CallFunction|IsIntEven (.x grid_index))) (Math|Float|SelectFloat 1.8e+02 0.0 (CallFunction|IsIntEven (.y grid_index))))))
    (else
      (return "0, 0, 0"))))

(fn GetTileLocationfromGridIndex
  (params (grid_index :type Int%20Point%20Structure))
  (return (+ (Variables|Default|Getgrid_bottom_left_corner_location) (* (Variables|Default|Getgrid_tile_size) (* grid_index (Utilities|Select :Index (Variables|Default|Getgrid_shape) :NewEnumerator0 "" :NewEnumerator1 "(X=1.000000,Y=1.000000)" :NewEnumerator2 "(X=0.750000,Y=0.500000)" :NewEnumerator3 "(X=1.000000,Y=0.500000)"))))))

(fn TraceforGround
  (params (tile_location :type Vector))
  (LocalVariables|Setradius (/ (.x (Variables|Default|Getgrid_tile_size)) (Math|Float|SelectFloat 5.0 3.0 (Utilities|Enum|Equal(Enum) (Variables|Default|Getgrid_shape) "NewEnumerator3"))))
  ;[1 1 1] take tile location +/-1000 and return all objects that collide with it in that range.
  (bind _outhits (Collision|MultiSphereTraceByChannel (+ tile_location "0.000000,0.000000,1000.000000") (- tile_location "0.000000,0.000000,1000.000000") (LocalVariables|Getradius) "TraceTypeQuery1" false 0 "None"))
  (if (> (Utilities|Array|Length _outhits) 0)
    (return true (Math|Vector|MakeVector (.x tile_location) (.y tile_location) (Math|Float|SnapToGrid(Float) (- (.Z (Math|Vector|BreakVector (.Location (Collision|BreakHitResult (Utilities|Array|Get(acopy) _outhits))))) (LocalVariables|Getradius)) (.z (Variables|Default|Getgrid_tile_size)))))
    (else
      (return false tile_location))))

(fn SetGridOffsetfromGround
  (params (offset :type Float%20%28double-precision%29))
  (Variables|Default|Setgrid_offset_from_ground offset)
  (Transformation|SetWorldLocation (Variables|Default|GetInstancedStaticMesh) (Math|Vector|MakeVector 0.0 0.0 (Variables|Default|Getgrid_offset_from_ground)) false false))