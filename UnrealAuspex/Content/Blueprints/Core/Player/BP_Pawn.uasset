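; BP_Pawn is a player pawn that acts as a movable camera rig with pan, stepped yaw rotation and spring arm zoom.
; Input events only update desired location, rotation and zoom values, with movement relative to the pawn's facing and zoom clamped to limits.
; Tick interpolates the actor transform and spring arm length toward those targets for smooth motion, moving without sweep collision.
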(event EventTick
  (params (DeltaSeconds :type Float%20%28single-precision%29))
  (bind _springarm (Variables|Default|GetSpringArm))
  (Variables|/Script/Engine.SpringArmComponent|SetTargetArmLength _springarm (Math|Interpolation|FInterpTo (Variables|/Script/Engine.SpringArmComponent|GetTargetArmLength _springarm) (Variables|Default|GetZoomDesired) DeltaSeconds (Variables|Default|Getzoom_interp)))
  (Transformation|SetActorLocation (Math|Interpolation|VInterpTo (Transformation|GetActorLocation) (Variables|Default|GetLocationDesired) DeltaSeconds (Variables|Default|Getlocation_interp)) false false)
  (Transformation|SetActorRotation (Math|Interpolation|RInterpTo (Transformation|GetActorRotation) (Variables|Default|GetRotationDesired) DeltaSeconds (Variables|Default|Getrotate_interp))))

(event EventBeginPlay
  (Variables|Default|SetLocationDesired (Transformation|GetActorLocation))
  (Variables|Default|SetZoomDesired (Variables|/Script/Engine.SpringArmComponent|GetTargetArmLength (Variables|Default|GetSpringArm)))
  (Variables|Default|SetRotationDesired (Transformation|GetActorRotation)))

(event Input|ActionEvents|InputActionInputAction_Left
  (params (Key :type Key%20Structure :default "None"))
  (:Pressed
    (Variables|Default|SetRotationDesired (Math|Rotator|CombineRotators (Variables|Default|GetRotationDesired) (Math|Rotator|MakeRotator 0.0 0.0 (Variables|Default|Getrotation_speed))))))

(event Input|ActionEvents|InputActionInputAction_Right
  (params (Key :type Key%20Structure :default "None"))
  (:Pressed
    (Variables|Default|SetRotationDesired (Math|Rotator|CombineRotators (Variables|Default|GetRotationDesired) (Math|Rotator|MakeRotator 0.0 0.0 (- 0.0 (Variables|Default|Getrotation_speed)))))))

(event Input|AxisEvents|InputAxisInputAxis_Zoom
  (params (AxisValue :type Float%20%28single-precision%29))
  (Variables|Default|SetZoomDesired (Math|Float|Clamp(Float) (+ (Variables|Default|GetZoomDesired) (* AxisValue (Variables|Default|Getzoom_speed))) (Variables|Default|Getzoom_min) (Variables|Default|Getzoom_max))))

(event Input|AxisEvents|InputAxisInputAxis_Forward
  (params (AxisValue :type Float%20%28single-precision%29))
  (Variables|Default|SetLocationDesired (+ (Variables|Default|GetLocationDesired) (* (* AxisValue (- 0.0 (Variables|Default|Getlocation_speed))) (Transformation|GetActorForwardVector)))))

(event Input|AxisEvents|InputAxisInputAxis_Right
  (params (AxisValue :type Float%20%28single-precision%29))
  (Variables|Default|SetLocationDesired (+ (Variables|Default|GetLocationDesired) (* (* AxisValue (Variables|Default|Getlocation_speed)) (Transformation|GetActorRightVector)))))

(fn ConstructionScript)