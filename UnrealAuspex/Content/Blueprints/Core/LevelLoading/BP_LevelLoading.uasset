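; BP_LevelLoading keeps one streaming sublevel active at a time, tracked by name in LevelLoaded.
; On BeginPlay it force-loads the initial LevelLoaded value.
; LoadLevel skips repeat requests unless forced, clears the load and visibility flags on the current streaming level, then sets them on the new one.
; An invalid name other than "None" prints a red error.
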(event EventBeginPlay
  (CallFunction|LoadLevel (Variables|Default|Getlevel_loaded) true))

(fn ConstructionScript)

(fn LoadLevel
  (params (level :type String) (force :type Boolean))
  (if (or force (Utilities|Enum|NotEqual(Enum) level (Variables|Default|Getlevel_loaded)))
    (Utilities|FlowControl|Sequence
      (:then_0
        (Utilities|IsValid (Class|GameplayStatics|GetStreamingLevel (Utilities|String|StringToName (Variables|Default|Getlevel_loaded)))
          (:Is%20Valid
            (Variables|/Script/Engine.LevelStreaming|SetbShouldBeLoaded (Class|GameplayStatics|GetStreamingLevel (Utilities|String|StringToName (Variables|Default|Getlevel_loaded))) false)
            (Variables|/Script/Engine.LevelStreaming|SetbShouldBeVisible (Class|GameplayStatics|GetStreamingLevel (Utilities|String|StringToName (Variables|Default|Getlevel_loaded))) false))))
      (:then_1
        (bind _output_get (Variables|Default|Setlevel_loaded level))
        (Utilities|IsValid (Class|GameplayStatics|GetStreamingLevel (Utilities|String|StringToName _output_get))
          (:Is%20Valid
            (Variables|/Script/Engine.LevelStreaming|SetbShouldBeLoaded (Class|GameplayStatics|GetStreamingLevel (Utilities|String|StringToName _output_get)) true)
            (Variables|/Script/Engine.LevelStreaming|SetbShouldBeVisible (Class|GameplayStatics|GetStreamingLevel (Utilities|String|StringToName _output_get)) true))
          (:Is%20Not%20Valid
            (if (Utilities|Enum|NotEqual(Enum) (Variables|Default|Getlevel_loaded) "None")
              (Development|PrintString (Utilities|String|Append "Error: LoadLevel - invalid level name [" (Variables|Default|Getlevel_loaded) "]") true true "(R=0.960000,G=0.000000,B=0.000000,A=1.000000)"))))))))